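; Pickup item actor that characters can interact with to add it to their inventory.
; Interact passes one of its ItemStructure to the interacter's InventoryComponent and destroys the actor if that succeeds.
; Its box overlap with a ChildCharacterBP shows a pickup widget at the character's projected screen position, gated by a DoOnce that resets when overlap ends.
; UseItem simply returns true.
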(event OnComponentBeginOverlap(Box)
  (params (OverlappedComponent :type Primitive%20Component%20Object%20Reference) (OtherActor :type Actor%20Object%20Reference) (OtherComp :type Primitive%20Component%20Object%20Reference) (OtherBodyIndex :type Integer) (bFromSweep :type Boolean) (SweepResult :type Hit%20Result%20Structure%20%28by%20ref%29))
  (bind _aschild_character_bp (Utilities|Casting|CastToChildCharacterBP OtherActor))
  (Variables|Default|SetScreen%20Location (.ScreenLocation (Class|PlayerController|ProjectWorldLocationtoScreen (Game|GetPlayerController 0) (Transformation|GetActorLocation _aschild_character_bp) false)))
  (Utilities|FlowControl|DoOnce false
    (:Completed
      (bind _returnvalue (UserInterface|CreateWidget "/Game/BluePrints/InventorySystem/InventoryUI/PickUpWidget.PickUpWidget_C" (Game|GetPlayerController 0)))
      (bind _output_get (Variables|Default|SetWidgetRef _returnvalue))
      (UserInterface|Viewport|AddtoViewport _output_get 0)
      (Class|UserWidget|SetAlignmentinViewport _output_get "(X=1.000000,Y=1.000000)")
      (Class|UserWidget|SetPositioninViewport _output_get (Variables|Default|GetScreen%20Location) true))))

(event OnComponentEndOverlap(Box)
  (params (OverlappedComponent :type Primitive%20Component%20Object%20Reference) (OtherActor :type Actor%20Object%20Reference) (OtherComp :type Primitive%20Component%20Object%20Reference) (OtherBodyIndex :type Integer))
  (Utilities|Casting|CastToChildCharacterBP OtherActor)
  (bind _widgetref (Variables|Default|GetWidgetRef)
    (:then
      (Widget|RemovefromParent _widgetref)
      (Variables|Default|SetWidgetRef 0)
      (Utilities|FlowControl|DoOnce false) ; enters at Reset
    )
    (:else)))

(event EventInteract
  (params (Interacter :type Actor%20Object%20Reference))
  ;[1 1 1] When you interact with an item that can be interacted with -> add it to your inventory.
  (bind _success (Default|AddtoInventory (Actor|GetComponentbyClass Interacter "/Game/BluePrints/InventorySystem/InventoryComponent.InventoryComponent_C") (Utilities|Struct|MakeSlotStructure (Variables|Default|GetItemStructure) 1)))
  (if _success
    (Development|PrintString "Added To Inventory")
    (Actor|DestroyActor)))

(fn ConstructionScript)

(fn UseItem
  (return true))