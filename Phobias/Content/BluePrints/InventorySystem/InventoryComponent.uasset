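; Inventory component that stores item stacks in a slot array sized on BeginPlay and toggles an inventory window.
; AddToInventory tops up a partial stack of the same item class for stackable items, otherwise it creates a new stack.
; AddToStack caps overfilled stacks and passes a remainder back to AddToInventory as non-stackable.
; ToggleInventory adds or removes the centre-anchored widget on the HUD canvas, switching input mode and mouse cursor.
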(event EventBeginPlay
  (Development|PrintString "Pre Prepare")
  (CallFunction|PrepareInventory)
  (Development|PrintString "Whats Next"))

(fn ToggleInventory
  (bind _returnvalue (Game|GetPlayerController 0))
  (bind _returnvalue_2 (Game|GetPlayerController 0))
  (Variables|Default|GetInventoryWindow
    (:then
      (Widget|RemovefromParent (Variables|Default|GetInventoryWindow))
      (Variables|Default|SetInventoryWindow 0)
      (Input|SetInputModeGameOnly _returnvalue)
      (Variables|/Script/Engine.PlayerController|SetbShowMouseCursor _returnvalue false))
    (:else
      (bind _returnvalue_3 (UserInterface|CreateWidget "/Game/BluePrints/InventorySystem/InventoryUI/InventoryWindow.InventoryWindow_C" 0 self))
      (Variables|Default|SetInventoryWindow _returnvalue_3)
      (bind _aschar_player_controller (Utilities|Casting|CastToCharPlayerController _returnvalue))
      (bind _returnvalue_4 (Class|CanvasPanel|AddChildtoCanvas (Variables|/Game/BluePrints/InventorySystem/InventoryUI/HUD.HUD_C|GetHUDCanvas (Variables|/Game/CharPlayerController.CharPlayerController_C|GetHudWidget _aschar_player_controller)) (Variables|Default|GetInventoryWindow)))
      (Class|CanvasPanelSlot|SetAutoSize _returnvalue_4 true)
      (Class|CanvasPanelSlot|SetAlignment _returnvalue_4 "(X=0.500000,Y=0.500000)")
      (Class|CanvasPanelSlot|SetAnchors _returnvalue_4 (Utilities|Struct|MakeAnchors "(X=0.500000,Y=0.500000)" "(X=0.500000,Y=0.500000)"))
      (Class|CanvasPanelSlot|SetPosition _returnvalue_4 (Variables|Default|GetPosition))
      (Input|SetInputModeUIOnly _returnvalue_2 (Variables|Default|GetInventoryWindow) "LockAlways")
      (Variables|/Script/Engine.PlayerController|SetbShowMouseCursor _returnvalue_2 true))))

(fn AddtoInventory
  (params (ContentToAdd :type Slot%20Structure%20Structure) (ContentToAdd_ItemStructure_IsStackable? :type Boolean))
  (if ContentToAdd_ItemStructure_IsStackable?
    (Development|PrintString "Add True")
    (bind _stackindex (Utilities|HasPartialStack ContentToAdd)
      (:True
        (CallFunction|AddtoStack ContentToAdd _stackindex))
      (:False
        (CallFunction|CreateStack ContentToAdd :!label _label)))
    (else
      (Development|PrintString "Add False")
      (goto _label)))
  (Development|PrintString "Add")
  (return true))

(fn PrepareInventory
  (Utilities|Array|Resize (Variables|Default|GetInventory) (Variables|Default|GetNumberOfSlots))
  (Development|PrintString "Prepared"))

(fn CreateStack
  (params (ContentToAdd :type Slot%20Structure%20Structure))
  (bind _inventory (Variables|Default|GetInventory))
  (Utilities|Array|SetArrayElem :TargetArray _inventory :Index (Utilities|Array|FindItem :TargetArray _inventory))
  (Development|PrintString "Create"))

(fn AddtoStack
  (params (SlotStruct :type Slot%20Structure%20Structure) (SlotIndex :type Integer))
  (bind _inventory (Variables|Default|GetInventory))
  (bind _inventory_2 (Variables|Default|GetInventory))
  (bind (_output _output_itemstructure_maxstacksize) (Utilities|Array|Get(acopy) _inventory SlotIndex))
  (bind _output_2 (Utilities|Array|Get(acopy) _inventory_2 SlotIndex))
  (Development|PrintString "Adding To Stack")
  (bind _output_get (LocalVariables|SetCurrentQuantity (.quantity _output)))
  (if (> (+ _output_get (.Quantity (Utilities|Struct|BreakSlotStructure SlotStruct))) _output_itemstructure_maxstacksize)
    (Utilities|Array|SetArrayElem (Variables|Default|GetInventory) SlotIndex (Utilities|Struct|MakeSlotStructure (.itemstructure SlotStruct) (.MaxStackSize (Utilities|Struct|BreakItemStructure (.itemstructure SlotStruct)))))
    (CallFunction|AddtoInventory (Utilities|Struct|MakeSlotStructure (.itemstructure SlotStruct) (- (.quantity SlotStruct) (LocalVariables|GetCurrentQuantity))) false)
    (else
      (Utilities|Array|SetArrayElem (Variables|Default|GetInventory) SlotIndex (Utilities|Struct|MakeSlotStructure (.itemstructure _output_2) (+ (.quantity _output_2) (.quantity SlotStruct))))))
  (return))