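; Courage potion item for the inventory system that raises the player's Courage when used.
; UseItem runs the parent logic, then casts the player character to ChildCharacterBP and calls AddToPlayerCourage only if Courage is below its cap.
; It returns CouragePotionUsable to report whether the potion could be used.
; The event graph holds only disabled placeholder events.
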(event EventBeginPlay)

(event Collision|EventActorBeginOverlap
  (params (OtherActor :type Actor%20Object%20Reference)))

(event EventTick
  (params (DeltaSeconds :type Float%20%28single-precision%29)))

(fn ConstructionScript
  (|CallParentFunction))

(fn UseItem
  (bind _returnvalue (Game|GetPlayerCharacter 0))
  (bind _aschild_character_bp (Utilities|Casting|CastToChildCharacterBP _returnvalue))
  (|CallParentFunction)
  (if (< (Variables|/Game/ThirdPersonBP/Blueprints/ChildCharacterBP.ChildCharacterBP_C|GetCourage _aschild_character_bp) 100)
    (LocalVariables|SetCouragePotionUsable? true)
    (Default|AddtoPlayerCourage _aschild_character_bp)
    (else
      (LocalVariables|SetCouragePotionUsable? false)))
  (return (LocalVariables|GetCouragePotionUsable?)))