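; Interactable door that can require a colored key, swinging open or closed on a timeline that rotates its pivot.
; Overlap checks the player's owned keys and shows a screen-projected open or missing-key widget; overlapping an unlocked door also drives the swing.
; Interacting with the matching key clears the requirement, removes the key and saves the remaining keys to the game instance.
; The construction script sets the door material from its color.
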(event OnComponentBeginOverlap(Overlap)
  (params (OverlappedComponent :type Primitive%20Component%20Object%20Reference) (OtherActor :type Actor%20Object%20Reference) (OtherComp :type Primitive%20Component%20Object%20Reference) (OtherBodyIndex :type Integer) (bFromSweep :type Boolean) (SweepResult :type Hit%20Result%20Structure%20%28by%20ref%29))
  ;[1 1 1] When player overlaps with door. Loop through player's owned keys array. If they have the key, set variable to true.
  (if (Variables|Default|GetIsKeyRequired?)
    (bind _aschild_character_bp (Utilities|Casting|CastToChildCharacterBP OtherActor))
    (for (_array_element _array_index) (Variables|/Game/ThirdPersonBP/Blueprints/ChildCharacterBP.ChildCharacterBP_C|GetOwnedKeys _aschild_character_bp)
      (if (Utilities|Enum|Equal(Enum) _array_element (Variables|Default|GetRequiredKeyType))
        (Variables|Default|SetPlayerHasKey? true)
        (else
          (Variables|Default|SetPlayerHasKey? false))))
    (Variables|Default|SetScreen%20Location (.ScreenLocation (Class|PlayerController|ProjectWorldLocationtoScreen (Game|GetPlayerController 0) (Transformation|GetActorLocation) false)))
    (Utilities|FlowControl|DoOnce false :!label _label
      (:Completed
        (CallFunction|CreateWidget)))
    (else
      ;[1 1 1] Is Key Still Required?
      (if (Variables|Default|GetIsKeyRequired?)
        ;[1 1 1] Does the player have the key?
        (if (Variables|Default|GetPlayerHasKey?)
          ;[1 1 1] On first use of key. Set key requirement off
          (Variables|Default|SetIsKeyRequired? false)
          (Utilities|FlowControl|Sequence
            (:then_0
              ;[1 1 1] Will Decide how the rotation
              (if (Variables|Default|GetisDoorClosed?) :!label _label_2
                (bind _doormovement (Timeline|DoorMovement Play)
                  (:Update
                    (Transformation|SetWorldRotation (Variables|Default|GetPivot) (Math|Rotator|MakeRotator 0.0 0.0 (Math|Float|Lerp (Variables|Default|GetDoorRotationOpen) (Variables|Default|GetDoorRotationClose) _doormovement)) false false)
                    (if (Variables|Default|GetisDoorClosed?)
                      (Variables|Default|SetisDoorClosed? false)
                      ;[1 1 1] Remove Widget when you open the door . Since you cant open an open door...
                      (CallFunction|RemoveWidget)
                      (goto _label Reset)
                      (else
                        (Variables|Default|SetisDoorClosed? true)
                        (CallFunction|RemoveWidget)))))
                (else
                  (Timeline|DoorMovement Reverse))))
            (:then_1
              ;[1 1 1] Removes Key
              (Utilities|Array|RemoveIndex (Variables|/Game/ThirdPersonBP/Blueprints/ChildCharacterBP.ChildCharacterBP_C|GetOwnedKeys _aschild_character_bp) _array_index)
              ;[1 1 1] Remove key and save to game instance.
              (bind _asphobias_game_instance (Utilities|Casting|CastToPhobias_Game_Instance (Game|GetGameInstance)))
              (Variables|/Game/Phobias_Game_Instance.Phobias_Game_Instance_C|SetPlayerKeys _asphobias_game_instance (Variables|/Game/ThirdPersonBP/Blueprints/ChildCharacterBP.ChildCharacterBP_C|GetOwnedKeys _aschild_character_bp)))))
        (else
          (goto _label_2))))))

(event OnComponentEndOverlap(Overlap)
  (params (OverlappedComponent :type Primitive%20Component%20Object%20Reference) (OtherActor :type Actor%20Object%20Reference) (OtherComp :type Primitive%20Component%20Object%20Reference) (OtherBodyIndex :type Integer))
  (Utilities|Casting|CastToChildCharacterBP OtherActor)
  (CallFunction|RemoveWidget)
  (Utilities|FlowControl|DoOnce false) ; enters at Reset
)

(event Custom|OpenUp
  ;[1 1 1] Is Key Still Required?
  (if (Variables|Default|GetIsKeyRequired?)
    ;[1 1 1] Does the player have the key?
    (if (Variables|Default|GetPlayerHasKey?)
      ;[1 1 1] On first use of key. Set key requirement off
      (Variables|Default|SetIsKeyRequired? false)
      (Utilities|FlowControl|Sequence
        (:then_0
          ;[1 1 1] Will Decide how the rotation
          (if (Variables|Default|GetisDoorClosed?) :!label _label
            (bind _doormovement (Timeline|DoorMovement Play)
              (:Update
                (Transformation|SetWorldRotation (Variables|Default|GetPivot) (Math|Rotator|MakeRotator 0.0 0.0 (Math|Float|Lerp (Variables|Default|GetDoorRotationOpen) (Variables|Default|GetDoorRotationClose) _doormovement)) false false)
                (if (Variables|Default|GetisDoorClosed?)
                  (Variables|Default|SetisDoorClosed? false)
                  ;[1 1 1] Remove Widget when you open the door . Since you cant open an open door...
                  (CallFunction|RemoveWidget)
                  (Utilities|FlowControl|DoOnce false) ; enters at Reset
                  (else
                    (Variables|Default|SetisDoorClosed? true)
                    (CallFunction|RemoveWidget)))))
            (else
              (Timeline|DoorMovement Reverse))))
        (:then_1
          ;[1 1 1] Removes Key
          (Utilities|Array|RemoveIndex (Variables|/Game/ThirdPersonBP/Blueprints/ChildCharacterBP.ChildCharacterBP_C|GetOwnedKeys (stale OnComponentBeginOverlap(Overlap) _aschild_character_bp)) (stale OnComponentBeginOverlap(Overlap) _array_index))
          ;[1 1 1] Remove key and save to game instance.
          (bind _asphobias_game_instance (Utilities|Casting|CastToPhobias_Game_Instance (Game|GetGameInstance)))
          (Variables|/Game/Phobias_Game_Instance.Phobias_Game_Instance_C|SetPlayerKeys _asphobias_game_instance (Variables|/Game/ThirdPersonBP/Blueprints/ChildCharacterBP.ChildCharacterBP_C|GetOwnedKeys (stale OnComponentBeginOverlap(Overlap) _aschild_character_bp))))))
    (else
      (goto _label))))

(event EventInteract
  (params (Interacter :type Actor%20Object%20Reference))
  ;[1 1 1] Interact Interface
  (Utilities|Casting|CastToChildCharacterBP Interacter)
  (CallFunction|OpenUp))

(event EventBeginPlay
  ;[1 1 1] Checks on start up whether key is required or not.
  (if (Utilities|Enum|Equal(Enum) (Variables|Default|GetRequiredKeyType) "NewEnumerator0")
    (Variables|Default|SetIsKeyRequired? false)
    (else
      (Variables|Default|SetIsKeyRequired? true))))

(fn ConstructionScript
  (Rendering|Material|SetMaterial (Variables|Default|GetDoor) 0 (Utilities|Select :Index (Variables|Default|GetDoorColor) :NewEnumerator0 0 :NewEnumerator1 "/Game/BluePrints/KeySystem/Door+KeyMats/Yellow_Key_Mat.Yellow_Key_Mat" :NewEnumerator2 "/Game/BluePrints/KeySystem/Door+KeyMats/Red_Key_Mat.Red_Key_Mat" :NewEnumerator3 "/Game/BluePrints/KeySystem/Door+KeyMats/Blue_Key_Mat.Blue_Key_Mat" :NewEnumerator4 "/Game/BluePrints/KeySystem/Door+KeyMats/Green_Key_Mat.Green_Key_Mat")))

(fn CreateWidget
  (bind _returnvalue (Game|GetPlayerController 0))
  ;[1 1 1] What kind of widget will we create?
  (if (Variables|Default|GetIsKeyRequired?)
    (if (Variables|Default|GetPlayerHasKey?)
      ;[1 1 1] Player has the key, or the door has already been unlocked.
      (bind _returnvalue_2 (UserInterface|CreateWidget "/Game/BluePrints/KeySystem/MissingUI/OpenWidget.OpenWidget_C" _returnvalue :!label _label))
      (bind _output_get (Variables|Default|SetOpenWidgetRef _returnvalue_2))
      (UserInterface|Viewport|AddtoViewport _output_get 0)
      (Class|UserWidget|SetAlignmentinViewport _output_get "(X=1.000000,Y=1.000000)")
      (Class|UserWidget|SetPositioninViewport _output_get (Variables|Default|GetScreen%20Location) true)
      (else
        ;[1 1 1] Key is still required, and player is still missing a key
        (bind _returnvalue_3 (UserInterface|CreateWidget "/Game/BluePrints/KeySystem/MissingUI/MissingKeyWidget.MissingKeyWidget_C" _returnvalue))
        (bind _output_get_2 (Variables|Default|SetMissingWidgetRef _returnvalue_3))
        (UserInterface|Viewport|AddtoViewport _returnvalue_3 0)
        (Class|UserWidget|SetAlignmentinViewport _output_get_2 "(X=1.000000,Y=1.000000)")
        (Class|UserWidget|SetPositioninViewport _output_get_2 (Variables|Default|GetScreen%20Location) true)))
    (elif (Variables|Default|GetisDoorClosed?)
      (goto _label)
      (else
        (bind _returnvalue_4 (UserInterface|CreateWidget "/Game/BluePrints/KeySystem/MissingUI/CloseWidget.CloseWidget_C" _returnvalue))
        (bind _output_get_3 (Variables|Default|SetCloseWidgetRef _returnvalue_4))
        (UserInterface|Viewport|AddtoViewport _output_get_3 0)
        (Class|UserWidget|SetAlignmentinViewport _output_get_3 "(X=1.000000,Y=1.000000)")
        (Class|UserWidget|SetPositioninViewport _output_get_3 (Variables|Default|GetScreen%20Location) true)))))

(fn RemoveWidget
  (bind _missingwidgetref (Variables|Default|GetMissingWidgetRef)
    (:then
      (Widget|RemovefromParent _missingwidgetref)
      (Variables|Default|SetMissingWidgetRef 0))
    (:else
      (bind _openwidgetref (Variables|Default|GetOpenWidgetRef)
        (:then
          (Widget|RemovefromParent _openwidgetref)
          (Variables|Default|SetOpenWidgetRef 0))
        (:else
          (bind _closewidgetref (Variables|Default|GetCloseWidgetRef)
            (:then
              (Widget|RemovefromParent _closewidgetref)
              (Variables|Default|SetCloseWidgetRef 0))
            (:else)))))))