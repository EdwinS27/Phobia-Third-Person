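; BlinkingLights is a lighting Blueprint that blinks whatever is attached under its root component.
; From BeginPlay it runs an endless Delay loop that toggles DefaultSceneRoot visibility, propagating the change to child components.
; Each cycle makes two blinks that share LightRemainsOffDuration, followed by separate FirstDelay and SecondDelay gaps to give an uneven rhythm.
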(event EventBeginPlay
  (bind _defaultsceneroot (Variables|Default|GetDefaultSceneRoot))
  (Rendering|ToggleVisibility _defaultsceneroot true :!label _label)
  (Utilities|FlowControl|Delay (Variables|Default|GetLightRemainsOffDuration))
  (Rendering|ToggleVisibility _defaultsceneroot true)
  (Utilities|FlowControl|Delay (Variables|Default|GetFirstDelay))
  (Rendering|ToggleVisibility _defaultsceneroot true)
  (Utilities|FlowControl|Delay (Variables|Default|GetLightRemainsOffDuration))
  (Rendering|ToggleVisibility _defaultsceneroot true)
  (Utilities|FlowControl|Delay (Variables|Default|GetSecondDelay))
  (goto _label))

(fn ConstructionScript)