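; RuneBP is a collectible elemental rune pickup that grants its type to the player's character.
; The construction script picks the mesh from RuneType (Air, Fire, Earth or Water) and the material from a separate RuneMat selector.
; When a ChildCharacterBP overlaps the sphere, the rune adds its RuneType to that character's OwnedRunes and destroys itself.
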(event OnComponentBeginOverlap(Sphere)
  (params (OverlappedComponent :type Primitive%20Component%20Object%20Reference) (OtherActor :type Actor%20Object%20Reference) (OtherComp :type Primitive%20Component%20Object%20Reference) (OtherBodyIndex :type Integer) (bFromSweep :type Boolean) (SweepResult :type Hit%20Result%20Structure%20%28by%20ref%29))
  (bind _aschild_character_bp (Utilities|Casting|CastToChildCharacterBP OtherActor))
  (Utilities|Array|Add (Variables|/Game/ThirdPersonBP/Blueprints/ChildCharacterBP.ChildCharacterBP_C|GetOwnedRunes _aschild_character_bp) (Variables|Default|GetRuneType))
  (Actor|DestroyActor))

(event EventBeginPlay)

(fn ConstructionScript
  (Components|StaticMesh|SetStaticMesh (Variables|Default|GetRuneTypeMesh) (Utilities|Select :Index (Variables|Default|GetRuneType) :NewEnumerator0 "/Game/BluePrints/RuneSystem/RuneMesh/RuneAirMesh.RuneAirMesh" :NewEnumerator1 "/Game/BluePrints/RuneSystem/RuneMesh/RuneFireMesh.RuneFireMesh" :NewEnumerator2 "/Game/BluePrints/RuneSystem/RuneMesh/RuneEarthMesh.RuneEarthMesh" :NewEnumerator3 "/Game/BluePrints/RuneSystem/RuneMesh/RunWaterMesh.RunWaterMesh"))
  (Rendering|Material|SetMaterial (Variables|Default|GetRuneTypeMesh) 0 (Utilities|Select :Index (Variables|Default|GetRuneMat) :NewEnumerator0 "/Game/Meshes/Runes/Materials/Air.Air" :NewEnumerator1 "/Game/Meshes/Runes/Materials/Earth.Earth" :NewEnumerator2 "/Game/Meshes/Runes/Materials/Fire.Fire" :NewEnumerator3 "/Game/Meshes/Runes/Materials/Water.Water")))