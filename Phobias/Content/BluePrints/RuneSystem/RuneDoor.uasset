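; Rune-locked door that swings on its pivot once the player holds all four required runes.
; Overlap checks the character's OwnedRunes to set per-rune flags, which Tick combines into PlayerHasAllRunes.
; OpenUp plays or reverses a yaw Timeline based on IsDoorClosed, which flips on every Timeline update, or prints a missing-rune message.
; The Construction Script sets the door material from DoorColor.
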(event OnComponentBeginOverlap(Overlap)
  (params (OverlappedComponent :type Primitive%20Component%20Object%20Reference) (OtherActor :type Actor%20Object%20Reference) (OtherComp :type Primitive%20Component%20Object%20Reference) (OtherBodyIndex :type Integer) (bFromSweep :type Boolean) (SweepResult :type Hit%20Result%20Structure%20%28by%20ref%29))
  (bind _aschild_character_bp (Utilities|Casting|CastToChildCharacterBP OtherActor))
  (for _array_element (Variables|/Game/ThirdPersonBP/Blueprints/ChildCharacterBP.ChildCharacterBP_C|GetOwnedRunes _aschild_character_bp)
    (Utilities|FlowControl|Sequence
      (:then_0
        (if (Utilities|Enum|Equal(Enum) _array_element (Variables|Default|GetRequiredRune1))
          (Variables|Default|SetHasRune1? true)))
      (:then_1
        (if (Utilities|Enum|Equal(Enum) _array_element (Variables|Default|GetRequiredRune2))
          (Variables|Default|SetHasRune2? true)))
      (:then_2
        (if (Utilities|Enum|Equal(Enum) _array_element (Variables|Default|GetRequiredRune3))
          (Variables|Default|SetHasRune3? true)))
      (:then_3
        (if (Utilities|Enum|Equal(Enum) _array_element (Variables|Default|GetRequiredRune4))
          (Variables|Default|SetHasRune4? true))))))

(event Custom|OpenUp
  (if (Variables|Default|GetPlayerHasAllRunes?)
    (if (Variables|Default|GetisDoorClosed?)
      (bind _doormovement (Timeline|DoorMovement Play)
        (:Update
          (Transformation|SetWorldRotation (Variables|Default|GetPivot) (Math|Rotator|MakeRotator 0.0 0.0 (Math|Float|Lerp (Variables|Default|GetDoorRotationOpen) (Variables|Default|GetDoorRotationClose) _doormovement)) false false)
          (if (Variables|Default|GetisDoorClosed?)
            (Variables|Default|SetisDoorClosed? false)
            (else
              (Variables|Default|SetisDoorClosed? true)))))
      (else
        (Timeline|DoorMovement Reverse)))
    (else
      ;[1 1 1] Can do widget here
      (Development|PrintString "Missing Rune"))))

(event EventTick
  (params (DeltaSeconds :type Float%20%28single-precision%29))
  (if (Variables|Default|GetHasRune1?)
    (if (Variables|Default|GetHasRune2?)
      (if (Variables|Default|GetHasRune3?)
        (if (Variables|Default|GetHasRune4?)
          (Variables|Default|SetPlayerHasAllRunes? true)
          (else
            (Variables|Default|SetPlayerHasAllRunes? false :!label _label)))
        (else
          (goto _label)))
      (else
        (goto _label)))
    (else
      (goto _label))))

(fn ConstructionScript
  (Rendering|Material|SetMaterial (Variables|Default|GetDoor) 0 (Utilities|Select :Index (Variables|Default|GetDoorColor) :NewEnumerator0 0 :NewEnumerator1 "/Game/BluePrints/KeySystem/Door+KeyMats/Yellow_Key_Mat.Yellow_Key_Mat" :NewEnumerator2 "/Game/BluePrints/KeySystem/Door+KeyMats/Red_Key_Mat.Red_Key_Mat" :NewEnumerator3 "/Game/BluePrints/KeySystem/Door+KeyMats/Blue_Key_Mat.Blue_Key_Mat" :NewEnumerator4 0)))