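; Monster Blueprint that shuttles its skeletal mesh back and forth and threatens the child character.
; A timeline offsets the mesh from its starting location, with a delayed self-call from Update flipping between Play and Reverse.
; Overlapping FearRange subtracts a set amount of the child's Courage, while overlapping InstantGameLoss triggers the child's game-over sequence.
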(event OnComponentBeginOverlap(FearRange)
  (params (OverlappedComponent :type Primitive%20Component%20Object%20Reference) (OtherActor :type Actor%20Object%20Reference) (OtherComp :type Primitive%20Component%20Object%20Reference) (OtherBodyIndex :type Integer) (bFromSweep :type Boolean) (SweepResult :type Hit%20Result%20Structure%20%28by%20ref%29))
  ;[1 1 1] Take a chunk of characters courage.
  (bind _aschild_character_bp (Utilities|Casting|CastToChildCharacterBP OtherActor))
  (Variables|/Game/ThirdPersonBP/Blueprints/ChildCharacterBP.ChildCharacterBP_C|SetCourage _aschild_character_bp (- (Variables|/Game/ThirdPersonBP/Blueprints/ChildCharacterBP.ChildCharacterBP_C|GetCourage _aschild_character_bp) (Variables|Default|GetFearAmountPerOverlap))))

(event OnComponentBeginOverlap(InstantGameLoss)
  (params (OverlappedComponent :type Primitive%20Component%20Object%20Reference) (OtherActor :type Actor%20Object%20Reference) (OtherComp :type Primitive%20Component%20Object%20Reference) (OtherBodyIndex :type Integer) (bFromSweep :type Boolean) (SweepResult :type Hit%20Result%20Structure%20%28by%20ref%29))
  ;[1 1 1] Game Over Sequence
  (bind _aschild_character_bp (Utilities|Casting|CastToChildCharacterBP OtherActor))
  (Default|GameOverSeq _aschild_character_bp))

(event Custom|MonsterMovement
  ;[1 1 1] Recursive Function to allow movement forward and back
  (bind _output_get (Variables|Default|SetMovementForward (not (Variables|Default|GetMovementForward))))
  ;;[1 0 0] Edit distance the monster travels in MonsterMovementForward
  (if _output_get
    (bind _change_objects_location (Timeline|MonsterMovementForward Play)
      (:Update
        (Transformation|SetWorldLocation (Variables|SkeletalMeshActor|GetSkeletalMeshComponent) (+ _change_objects_location (Variables|Default|GetMonstersLocation)) false false)
        (Utilities|FlowControl|Delay (Variables|Default|GetDurationBeforeReset))
        (CallFunction|MonsterMovement)))
    (else
      (Timeline|MonsterMovementForward Reverse))))

(event EventBeginPlay
  ;[1 1 1] Grab objects location on start and call recursive function
  (Variables|Default|SetMonstersLocation (Transformation|GetWorldLocation (Variables|SkeletalMeshActor|GetSkeletalMeshComponent)))
  (CallFunction|MonsterMovement))

(fn ConstructionScript)